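; EdgeMarkerRight is a navigation marker for a ledge edge that tells AI units how far away to jump to land on it.
; Its construction script pins it to a fixed Y plane.
; CalculateJumpDistance rejects units that cannot reach the height or are on the wrong X side, then solves the projectile quadratic for the later landing time.
; It returns that time times movement speed, minus a buffer, or a failure enum, including for excessive airtime.
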(event EventBeginPlay)

(event Collision|EventActorBeginOverlap
  (params (OtherActor :type Actor%20Object%20Reference)))

(event EventTick
  (params (DeltaSeconds :type Float%20%28single-precision%29)))

(fn ConstructionScript
  (bind _returnvalue (Transformation|GetActorLocation))
  (Transformation|SetActorLocation (Math|Vector|MakeVector (.x _returnvalue) 2.0 (.z _returnvalue)) false false))

(fn CalculateJumpDistance
  (params (UnitPosition :type Vector%20%28by%20ref%29) (JumpSpeed :type Float%20%28single-precision%29%20%28by%20ref%29) (MovementSpeed :type Float%20%28single-precision%29%20%28by%20ref%29))
  (Utilities|FlowControl|Sequence
    (:then_0
      ;[0 0.955 1] Initial Data Setup
      (LocalVariables|SetGravity (.z (Class|Actor|GetInputVectorAxisValue)))
      (bind _output_get (LocalVariables|SetDistanceToLedge (- UnitPosition (Transformation|GetActorLocation))))
      (LocalVariables|SetHeight (.z _output_get)))
    (:then_1
      ;[1 0.01036 0.02031] Calculate if AI can even jump high enough: d = -V^2 / 2a
      (bind _result (Math|Float|NegateFloat (Math|Float|Square JumpSpeed))
        (:%20%20
          (if (> (/ _result (* 2.0 (LocalVariables|GetGravity))) (LocalVariables|GetHeight))
            ;[1 0.01989 0] Check if on Correct side:
            (if (not (< (.x (LocalVariables|GetDistanceToLedge)) 0.0))
              (return 0.0 "NewEnumerator2"))
            (else
              (return 0.0 "NewEnumerator1"))))))
    (:then_2
      ;[0 1 0.3925] Calculate time required to land on ledge, using quadratic formula
      (bind _result_2 (Math|Float|NegateFloat JumpSpeed)
        (:%20%20
          (bind _output_get_2 (LocalVariables|SetTimeRequired (select (< (/ (- _result_2 (Math|Float|Sqrt (+ (Math|Float|Square JumpSpeed) (* (* (LocalVariables|GetGravity) 2.0) (LocalVariables|GetHeight))))) (LocalVariables|GetGravity)) (/ (+ _result_2 (Math|Float|Sqrt (+ (Math|Float|Square JumpSpeed) (* (* (LocalVariables|GetGravity) 2.0) (LocalVariables|GetHeight))))) (LocalVariables|GetGravity))) (/ (+ _result_2 (Math|Float|Sqrt (+ (Math|Float|Square JumpSpeed) (* (* (LocalVariables|GetGravity) 2.0) (LocalVariables|GetHeight))))) (LocalVariables|GetGravity)) (/ (- _result_2 (Math|Float|Sqrt (+ (Math|Float|Square JumpSpeed) (* (* (LocalVariables|GetGravity) 2.0) (LocalVariables|GetHeight))))) (LocalVariables|GetGravity)))))
          ;[1 0 0.009094] Check if time required is too long
          (if (not (< _output_get_2 (LocalVariables|GetMaximumTimeThreshold)))
            (return 0.0 "NewEnumerator3")))))
    (:then_3
      ;[1 0.9123 0.1124] Once Time is Calculated, use to calculate Distance required to land on edge
      (return (- (* (LocalVariables|GetTimeRequired) MovementSpeed) (LocalVariables|GetDistanceBuffer)) "NewEnumerator0"))))