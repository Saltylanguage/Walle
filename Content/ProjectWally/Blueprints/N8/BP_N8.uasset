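; BP_N8 is a character built to follow the player along the world X axis.
; BeginPlay caches the player pawn as BP_Player and sets movement mode to walking.
; FollowPlayer applies movement input toward the player when the X gap exceeds DistanceThreshold, but nothing in this file calls it and Tick is empty.
; An unconnected SetActorLocation node that would place N8 at a fixed offset from the player never runs.
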(event EventBeginPlay
  (Utilities|FlowControl|Sequence
    (:then_0
      (bind _asbp_player (Utilities|Casting|CastToBP_Player (Game|Player|GetPlayerPawn 0)))
      (Variables|Default|SetPlayer _asbp_player)
      (Pawn|Components|CharacterMovement|SetMovementMode (Variables|Character|GetCharacterMovement) "MOVE_Walking" 0))))

(event Collision|EventActorBeginOverlap
  (params (OtherActor :type Actor%20Object%20Reference)))

(event EventTick
  (params (DeltaSeconds :type Float%20%28single-precision%29)))

(fn ConstructionScript)

(fn FollowPlayer
  (bind _output_get (LocalVariables|SetCurrentDistance (- (.x (Transformation|GetActorLocation (Variables|Default|GetPlayer))) (.x (Transformation|GetActorLocation)))))
  (if (> (Math|Float|Absolute(Float) _output_get) (LocalVariables|GetDistanceThreshold))
    (Pawn|Input|AddMovementInput "1.000000, 0, 0" (select (> (LocalVariables|GetCurrentDistance) 0.0) 1.0 -1.0) false)))