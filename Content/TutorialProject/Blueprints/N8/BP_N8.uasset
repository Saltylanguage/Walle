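; BP_N8 is an actor that follows the player pawn at a fixed world-space offset along negative X.
; On BeginPlay it casts the player pawn to BP_Player, caches the reference and snaps next to it.
; Every Tick it teleport-free sets its location from the player's position, without sweeping, using a larger offset than the initial placement.
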(event EventBeginPlay
  (bind _asbp_player (Utilities|Casting|CastToBP_Player (Game|Player|GetPlayerPawn 0)))
  (bind _output_get (Variables|Default|SetPlayer _asbp_player))
  (bind _output_get_2 (Variables|Default|SetPlayerLocation (Transformation|GetActorLocation _output_get)))
  (Transformation|SetActorLocation (+ _output_get_2 (Math|Vector|MakeVector -1e+01 0.0 0.0)) false false))

(event Collision|EventActorBeginOverlap
  (params (OtherActor :type Actor%20Object%20Reference)))

(event EventTick
  (params (DeltaSeconds :type Float%20%28single-precision%29))
  (Transformation|SetActorLocation (+ (Transformation|GetActorLocation (Variables|Default|GetPlayer)) (Math|Vector|MakeVector -2e+01 0.0 0.0)) false false))

(fn ConstructionScript)