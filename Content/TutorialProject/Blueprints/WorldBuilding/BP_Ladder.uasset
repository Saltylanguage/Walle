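; BP_Ladder is a climbable ladder built from Paper2D sprites that the player can climb while overlapping its box.
; The construction script stacks rung sprites between bottom and top points, pins the actor's Y, sizes the trigger box and places a scaled mesh at the top.
; Box overlaps toggle BP_Player's climb state, and leaving also ends climbing and restores the mesh's collision.
; AllowDown re-enters the begin-overlap logic.
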(event OnComponentBeginOverlap(Box)
  (params (OverlappedComponent :type Primitive%20Component%20Object%20Reference) (OtherActor :type Actor%20Object%20Reference) (OtherComp :type Primitive%20Component%20Object%20Reference) (OtherBodyIndex :type Integer) (bFromSweep :type Boolean) (SweepResult :type Hit%20Result%20Structure%20%28by%20ref%29))
  (bind _asbp_player (Utilities|Casting|CastToBP_Player OtherActor))
  (Variables|/Game/TutorialProject/Blueprints/Player/BP_Player.BP_Player_C|SetCanClimb _asbp_player true))

(event OnComponentEndOverlap(Box)
  (params (OverlappedComponent :type Primitive%20Component%20Object%20Reference) (OtherActor :type Actor%20Object%20Reference) (OtherComp :type Primitive%20Component%20Object%20Reference) (OtherBodyIndex :type Integer))
  (bind _asbp_player (Utilities|Casting|CastToBP_Player OtherActor))
  (Variables|/Game/TutorialProject/Blueprints/Player/BP_Player.BP_Player_C|SetIsClimbing _asbp_player false)
  (Variables|/Game/TutorialProject/Blueprints/Player/BP_Player.BP_Player_C|SetCanClimb _asbp_player false)
  (Default|ClimbingEnd _asbp_player)
  (Collision|SetCollisionEnabled (Variables|Default|GetStaticMesh) "QueryAndPhysics"))

(event Custom|AllowDown
  (bind _asbp_player (Utilities|Casting|CastToBP_Player (stale OnComponentBeginOverlap(Box) OtherActor)))
  (Variables|/Game/TutorialProject/Blueprints/Player/BP_Player.BP_Player_C|SetCanClimb _asbp_player true))

(fn ConstructionScript
  (bind _self self)
  (bind _staticmesh (Variables|Default|GetStaticMesh))
  (bind _box (Variables|Default|GetBox))
  (bind _laddertop (Variables|Default|GetLadderTop))
  (bind _ladderbottom (Variables|Default|GetLadderBottom))
  (bind _rungoffset (Variables|Default|GetRungOffset))
  (bind _returnvalue (- _laddertop _ladderbottom))
  (bind _returnvalue_2 (Transformation|GetActorLocation _self))
  (bind _returnvalue_3 (/ (.z _returnvalue) 2.0))
  (Utilities|FlowControl|Sequence
    (:then_0
      (for _index (range 0 (Math|Float|Truncate (/ (.z _returnvalue) _rungoffset)))
        (bind _returnvalue_4 (AddComponent|AddPaperSpriteComponent false (Math|Transform|MakeTransform (Math|Vector|MakeVector 0.0 0.0 (* _index _rungoffset)) "0, 0, 0" "1,1,1")))
        (Rendering|Components|Sprite|SetSprite _returnvalue_4 (Variables|Default|GetLadderSprite))
        (Collision|SetCollisionEnabled _returnvalue_4 "NoCollision")
        (Transformation|SetActorLocation _self (Math|Vector|MakeVector (.x _returnvalue_2) -1.0 (.z _returnvalue_2)) false false))
      (Transformation|SetRelativeScale3D _box (Math|Vector|MakeVector (Variables|Default|GetCollisionWidth) 1.0 _returnvalue_3))
      (Transformation|SetRelativeLocation _box (Math|Vector|MakeVector 0.0 0.0 _returnvalue_3) false false))
    (:then_1
      (Transformation|SetRelativeScale3D _staticmesh (Math|Vector|MakeVector (Variables|Default|GetCollisionWidth) 2e+01 1.0))
      (Transformation|SetRelativeLocation _staticmesh (Variables|Default|GetLadderTop) false false))))