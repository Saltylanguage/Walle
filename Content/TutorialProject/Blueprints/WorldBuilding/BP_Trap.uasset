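; BP_Trap is a world trap that damages the player standing inside its Box volume.
; Every Tick it runs a box overlap query matching the Box's position and extent, filtered to WorldDynamic BP_Player actors.
; It casts the first result and calls DamageSystem with DamageVal, so damage repeats each frame during overlap.
; An alternative damage-on-begin-overlap chain is left disconnected and never runs.
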(event OnComponentBeginOverlap(Box)
  (params (OverlappedComponent :type Primitive%20Component%20Object%20Reference) (OtherActor :type Actor%20Object%20Reference) (OtherComp :type Primitive%20Component%20Object%20Reference) (OtherBodyIndex :type Integer) (bFromSweep :type Boolean) (SweepResult :type Hit%20Result%20Structure%20%28by%20ref%29)))

(event EventBeginPlay)

(event EventActorBeginOverlap
  (params (OtherActor :type Actor%20Object%20Reference)))

(event EventTick
  (params (DeltaSeconds :type Float%20%28single-precision%29))
  (bind _box (Variables|Default|GetBox))
  (bind _outactors (Class|KismetSystemLibrary|BoxOverlapActorsNEW (Transformation|GetWorldLocation _box) (Components|Box|GetScaledBoxExtent _box) (Utilities|Array|MakeArray "ObjectTypeQuery2") "/Game/TutorialProject/Blueprints/Player/BP_Player.BP_Player_C"))
  (bind _asbp_player (Utilities|Casting|CastToBP_Player (Utilities|Array|Get(acopy) _outactors)))
  (Default|DamageSystem _asbp_player (Variables|Default|GetDamage_Val)))

(fn ConstructionScript)