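; BP_ActivatedPlatform is a moving platform that travels between two points, PointA and PointB, when BP_Player overlaps its trigger Box.
; The overlap checks which endpoint the actor is at, using the platform's X scale as tolerance, and selects the opposite one as destination.
; LerpTimeline then drives a swept location lerp to that point, with its play rate derived from Time in the construction script.
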(event OnComponentBeginOverlap(Box)
  (params (OverlappedComponent :type Primitive%20Component%20Object%20Reference) (OtherActor :type Actor%20Object%20Reference) (OtherComp :type Primitive%20Component%20Object%20Reference) (OtherBodyIndex :type Integer) (bFromSweep :type Boolean) (SweepResult :type Hit%20Result%20Structure%20%28by%20ref%29))
  (bind _platformlength (Variables|Default|GetPlatformLength))
  ;[0 0.05436 1] When Player Overlaps Box, Move to Destination and Stop
  (bind _asbp_player (Utilities|Casting|CastToBP_Player OtherActor))
  (if (Math|Vector|Equal(Vector) (Transformation|GetActorLocation) (Transformation|GetActorLocation (Variables|Default|GetPoint%20A)) _platformlength)
    (Variables|Default|SetDesinationIndex 1)
    (bind _alphavalue (Timeline|LerpTimeline PlayFromStart)
      (:Update
        (Collision|IgnoreActorwhenMoving (Variables|Default|GetPlatform) _asbp_player false)
        (switch int (Variables|Default|GetDesinationIndex)
          (:Default
            (Transformation|SetActorLocation (Math|Vector|Lerp(Vector) (Transformation|GetActorLocation (Variables|Default|GetPoint%20B)) (Transformation|GetActorLocation (Variables|Default|GetPoint%20A)) _alphavalue) true false :!label _label))
          (:0
            (goto _label))
          (:1
            (Transformation|SetActorLocation (Math|Vector|Lerp(Vector) (Transformation|GetActorLocation (Variables|Default|GetPoint%20A)) (Transformation|GetActorLocation (Variables|Default|GetPoint%20B)) _alphavalue) true false)))))
    (elif (Math|Vector|Equal(Vector) (Transformation|GetActorLocation) (Transformation|GetActorLocation (Variables|Default|GetPoint%20B)) _platformlength)
      (Variables|Default|SetDesinationIndex 0)
      (Timeline|LerpTimeline PlayFromStart))))

(event EventBeginPlay
  (Variables|Default|SetPlatformLength (.x (Transformation|GetWorldScale (Variables|Default|GetPlatform)))))

(event Collision|EventActorBeginOverlap
  (params (OtherActor :type Actor%20Object%20Reference))
  ;[0 0.05436 1] When Player Overlaps Box, Move to Destination and Stop
)

(event EventTick
  (params (DeltaSeconds :type Float%20%28single-precision%29))
  ;[0 0.05436 1] When Player Overlaps Box, Move to Destination and Stop
)

(fn ConstructionScript
  (bind _output_get (Variables|Default|SetPlayrateModifier (/ 6e+01 (Variables|Default|GetTime))))
  (Components|Timeline|SetPlayRate (Variables|Default|GetLerpTimeline) _output_get))