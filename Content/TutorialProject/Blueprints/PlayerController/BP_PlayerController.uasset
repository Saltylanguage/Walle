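; Player controller for a 2D side-view character that handles mouse-aimed shooting and weapon cycling.
; Holding left mouse opens a gate on Tick, which spawns BP_Shot at the pawn's arrow once a tick counter reaches ShotDelay, given the Shoot upgrade and a selected weapon.
; Shots fly toward the deprojected cursor on the XZ plane.
; CycleWeaponUp loads WeaponData table rows, whose color, scale and speed apply to each shot.
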(event Custom|InitWeapon
  ;[1 0.04116 0.071] Switch Weapon Parameters
  (bind _outrownames (DataTable|GetDataTableRowNames "/Game/TutorialProject/Blueprints/Player/WeaponData.WeaponData"))
  (bind _output_get (Variables|Default|SetWeaponArray _outrownames))
  (Variables|Default|SetNumberOfWeapons (Utilities|Array|Length _output_get)))

(event EventBeginPlay
  ;[1 0.9937 0] Set Player Pawn
  (bind _asbp_player (Utilities|Casting|CastToBP_Player (Pawn|GetControlledPawn)))
  (Variables|Default|SetPlayerPawn _asbp_player)
  (CallFunction|InitWeapon))

(event EventTick
  (params (DeltaSeconds :type Float%20%28single-precision%29))
  (bind _worldlocation (Game|Player|ConvertMouseLocationToWorldSpace))
  (bind _playerpawn (Variables|Default|GetPlayerPawn))
  (bind _playerpawn_2 (Variables|Default|GetPlayerPawn))
  (bind _arrow (Variables|/Game/TutorialProject/Blueprints/Player/BP_Player.BP_Player_C|GetArrow _playerpawn_2))
  (bind _returnvalue (Transformation|GetWorldLocation _arrow))
  (bind _returnvalue_2 (Math|Transform|MakeTransform _returnvalue "0, 0,0.000000" "1.000000,1,1"))
  ;[1 0.04116 0.071] Handle Shoot
  (Variables|Default|SetX_Offset (* (Variables|/Game/TutorialProject/Blueprints/Player/BP_Player.BP_Player_C|GetFacing (Variables|Default|GetPlayerPawn)) (Variables|Default|GetX_Offset)))
  (if (>= (Variables|Default|GetCounter) (Variables|Default|GetShotDelay))
    (Utilities|FlowControl|Gate true
      (:Exit
        (bind _asbp_player (Utilities|Casting|CastToBP_Player (Game|Player|GetPlayerPawn 0)))
        (if (.shoot (Variables|/Game/TutorialProject/Blueprints/Player/BP_Player.BP_Player_C|GetUpgrades _asbp_player))
          (if (> (Variables|Default|GetWeaponIndex) 0)
            (Utilities|FlowControl|Delay 0.1)
            (if (Variables|/Game/TutorialProject/Blueprints/Player/BP_Player.BP_Player_C|GetIsJumping (Variables|Default|GetPlayerPawn))
              (Variables|Default|SetBulletTransform (Math|Transform|MakeTransform (Math|Vector|MakeVector (+ (.x (.location _returnvalue_2)) (Variables|Default|GetX_Offset)) (.y (.location _returnvalue_2)) (+ (.z (.location _returnvalue_2)) (Variables|Default|GetZ_Offset))) (.rotation _returnvalue_2) (.scale _returnvalue_2)))
              (else
                (Variables|Default|SetBulletTransform (Math|Conversions|ToTransform(Vector) _returnvalue))))
            (bind _returnvalue_3 (Game|SpawnActorfromClass "/Game/TutorialProject/Blueprints/Projectiles/BP_Shot.BP_Shot_C" (Variables|Default|GetBulletTransform) "Undefined" 0 0))
            (CallFunction|SetWeaponParameters _returnvalue_3)
            ;[0 1 0.1598] Pass Shoot Animation to Player Class
            (Variables|/Game/TutorialProject/Blueprints/Player/BP_Player.BP_Player_C|SetIsShooting (Variables|Default|GetPlayerPawn) true)
            (Variables|/Script/Engine.MovementComponent|SetVelocity (Variables|/Game/TutorialProject/Blueprints/Projectiles/BP_Shot.BP_Shot_C|GetProjectileMovement _returnvalue_3) (* (Math|Vector|Normalize (- (Math|Vector|MakeVector (.x _worldlocation) 0.0 (.z _worldlocation)) _returnvalue)) (Variables|/Script/Engine.ProjectileMovementComponent|GetInitialSpeed (Variables|/Game/TutorialProject/Blueprints/Projectiles/BP_Shot.BP_Shot_C|GetProjectileMovement _returnvalue_3))))
            (Variables|Default|SetCounter 0)
            (if (> (Math|Vector|VectorLength (Transformation|GetVelocity (Variables|Default|GetPlayerPawn))) 0.0)
              (Variables|/Game/TutorialProject/Blueprints/Player/BP_Player.BP_Player_C|SetisMoving _playerpawn true)
              (else
                (Variables|/Game/TutorialProject/Blueprints/Player/BP_Player.BP_Player_C|SetisMoving _playerpawn false)))))))
    (else
      (Variables|Default|SetCounter (+ (Variables|Default|GetCounter) 1 0))
      (Utilities|FlowControl|RetriggerableDelay 0.25)
      (Variables|/Game/TutorialProject/Blueprints/Player/BP_Player.BP_Player_C|SetIsShooting (Variables|Default|GetPlayerPawn) false))))

(event Input|ActionEvents|InputActionCycleWeaponUp
  (params (Key :type Key%20Structure :default "AnyKey"))
  ;[1 0.04116 0.071] Switch Weapon Parameters
  (:Pressed
    (Variables|Default|SetWeaponIndex (+ (Variables|Default|GetWeaponIndex) 1))
    (if (>= (Variables|Default|GetWeaponIndex) (Variables|Default|GetNumberOfWeapons))
      (Variables|Default|SetWeaponIndex 1)
      (Development|PrintString "Index = 0"))
    (CallFunction|InitWeapon)
    (Development|PrintString (Utilities|String|ToString(Integer) (Variables|Default|GetWeaponIndex)))
    (bind _returnvalue (Utilities|GetDataTableRow "/Game/TutorialProject/Blueprints/Player/WeaponData.WeaponData" (Utilities|Array|Get(acopy) (Variables|Default|GetWeaponArray) (Variables|Default|GetWeaponIndex)))
      (:then
        (Variables|Default|SetWeaponName (.name _returnvalue))
        (Variables|Default|SetWeaponColor (.color _returnvalue))
        (Variables|Default|SetWeaponVelocityX (.velocityx _returnvalue))
        (Variables|Default|SetWeaponVelocityZ (.velocityz _returnvalue))
        (Variables|Default|SetWeaponZRange (.velocityzrange _returnvalue))
        (Variables|Default|SetWeaponProjectileScale (.scale _returnvalue))
        (Variables|Default|SetWeaponFlipbook (.flipbook _returnvalue))
        (Development|PrintString (Variables|Default|GetWeaponName))
        (Development|PrintString (Utilities|String|ToString(Integer) (Variables|Default|GetWeaponColor))))
      (:RowNotFound
        (Development|PrintString "Couldn't Find Row")))))

(event Input|MouseEvents|LeftMouseButton
  (params (Key :type Key%20Structure :default "AnyKey"))
  (bind _worldlocation (Game|Player|ConvertMouseLocationToWorldSpace))
  (bind _playerpawn (Variables|Default|GetPlayerPawn))
  (bind _playerpawn_2 (Variables|Default|GetPlayerPawn))
  (bind _arrow (Variables|/Game/TutorialProject/Blueprints/Player/BP_Player.BP_Player_C|GetArrow _playerpawn_2))
  (bind _returnvalue (Transformation|GetWorldLocation _arrow))
  (bind _returnvalue_2 (Math|Transform|MakeTransform _returnvalue "0, 0,0.000000" "1.000000,1,1"))
  ;[1 0.04116 0.071] Handle Shoot
  (:Pressed
    (Variables|/Game/TutorialProject/Blueprints/Player/BP_Player.BP_Player_C|SetIsShooting (Variables|Default|GetPlayerPawn) true)
    (Utilities|FlowControl|Gate true) ; enters at Open
  )
  (:Released
    (Utilities|FlowControl|Gate true) ; enters at Close
  ))

(fn ConstructionScript)

(fn SetWeaponParameters
  (params (Weapon :type BP%20Shot%20Object%20Reference))
  (bind _weaponprojectilescale (Variables|Default|GetWeaponProjectileScale))
  (bind _output_get (Variables|Default|SetWeapon Weapon))
  (Rendering|Material|SetVectorParameterValue (Variables|/Game/TutorialProject/Blueprints/Projectiles/BP_Shot.BP_Shot_C|GetSpriteMaterial _output_get) "Color" (Variables|Default|GetWeaponColor) :!class /Script/Engine.MaterialInstanceDynamic)
  (Transformation|SetActorScale3D (Variables|Default|GetWeapon) (Math|Vector|MakeVector _weaponprojectilescale _weaponprojectilescale _weaponprojectilescale))
  (Variables|/Script/Engine.ProjectileMovementComponent|SetInitialSpeed (Variables|/Game/TutorialProject/Blueprints/Projectiles/BP_Shot.BP_Shot_C|GetProjectileMovement (Variables|Default|GetWeapon)) (Variables|Default|GetWeaponVelocityX))
  (return))