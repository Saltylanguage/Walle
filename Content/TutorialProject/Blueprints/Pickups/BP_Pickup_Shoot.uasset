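; BP_Pickup_Shoot is a pickup that unlocks the shooting upgrade for BP_Player.
; When the player overlaps its Box, it sets that upgrade in the player's Upgrades struct, preserving DoubleJump, and sets WeaponIndex on BP_PlayerController.
; It then destroys its flipbook sprite, shows a text message, and destroys itself after a short delay.
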(event OnComponentBeginOverlap(Box)
  (params (OverlappedComponent :type Primitive%20Component%20Object%20Reference) (OtherActor :type Actor%20Object%20Reference) (OtherComp :type Primitive%20Component%20Object%20Reference) (OtherBodyIndex :type Integer) (bFromSweep :type Boolean) (SweepResult :type Hit%20Result%20Structure%20%28by%20ref%29))
  (bind _asbp_player (Utilities|Casting|CastToBP_Player OtherActor))
  (Variables|/Game/TutorialProject/Blueprints/Player/BP_Player.BP_Player_C|SetUpgrades _asbp_player (Utilities|Struct|MakeUpgrades true (.doublejump (Variables|/Game/TutorialProject/Blueprints/Player/BP_Player.BP_Player_C|GetUpgrades _asbp_player))))
  (bind _asbp_player_controller (Utilities|Casting|CastToBP_PlayerController (Game|GetPlayerController 0)))
  (Variables|/Game/TutorialProject/Blueprints/PlayerController/BP_PlayerController.BP_PlayerController_C|SetWeaponIndex _asbp_player_controller 1)
  (Components|DestroyComponent (Variables|Default|GetPaperFlipbook))
  (Development|SetHiddeninGame (Variables|Default|GetTextRender) false false)
  (Utilities|FlowControl|Delay 3.0)
  (Actor|DestroyActor))

(event EventBeginPlay)

(event EventActorBeginOverlap
  (params (OtherActor :type Actor%20Object%20Reference)))

(event EventTick
  (params (DeltaSeconds :type Float%20%28single-precision%29)))

(fn ConstructionScript)